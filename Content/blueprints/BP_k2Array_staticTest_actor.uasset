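; Test actor that visualizes a texture as a grid of static mesh components, driven by K2A C++ functions.
; BeginPlay passes the texture to C++ and to a screen mesh's dynamic material, then spawns one scaled mesh per pixel block, sized by K2APxPerUnit, into an array.
; Each Tick, TransformArray updates that array from texture data using a depth scalar.
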(event `/Game/blueprints/BP_k2Array_dynamicTest_actor.ReceiveBeginPlay`
  (bind _k2a_texture (`self.k2A_texture`))
  (bind _k2a_pxperunit (`self.k2A_pxPerUnit`))
  (bind _k2a_gridscale (`self.k2A_gridScale`))
  (bind _returnvalue (/ (`Texture2D.Blueprint_GetSizeX` _k2a_texture) _k2a_pxperunit))
  (bind _returnvalue_2 (/ (`KismetMathLibrary.Conv_IntToDouble` _k2a_gridscale) (`KismetMathLibrary.Conv_IntToDouble` (`self.k2A_objScale`))))
  (`self.SetTexture` _k2a_texture) ; send texture to K2A C++ functions
  (`MaterialInstanceDynamic.SetTextureParameterValue` (`self.k2A_screenTxtrParam`) "dynamicTexture" _k2a_texture) ; send texture to screen object material
  (for _index (range (* (/ (`Texture2D.Blueprint_GetSizeY` _k2a_texture) _k2a_pxperunit) _returnvalue))
    (bind _returnvalue_3 (`AddComponent|StaticMeshComponent_22` :`RelativeTransform` (`KismetMathLibrary.MakeTransform` (`KismetMathLibrary.MakeVector` (`KismetMathLibrary.Conv_IntToDouble` (* (mod _index _returnvalue) _k2a_gridscale)) 500.0 (`KismetMathLibrary.Conv_IntToDouble` (* (/ _index _returnvalue) _k2a_gridscale))) (struct) (`KismetMathLibrary.MakeVector` _returnvalue_2 _returnvalue_2 _returnvalue_2)))) ; New static object
    (`KismetArrayLibrary.Array_Add` (`self.k2A_objArray`) _returnvalue_3) ; add new object to arrray
  ))

(event `self.ReceiveActorBeginOverlap`
  (params (OtherActor :type "Actor Object Reference")))

(event `/Game/blueprints/BP_k2Array_dynamicTest_actor.ReceiveTick`
  (params (DeltaSeconds :type "Float (single-precision)"))
  (`self.transform_Array` (`self.TextureData`) (`self.k2A_objArray`) (`self.k2A_verbose`) (`self.k2A_pxPerUnit`) (`self.k2A_depthScalar`)))

(fn `UserConstructionScript`
  (bind _returnvalue (`PrimitiveComponent.CreateDynamicMaterialInstance` (`self.screenMesh`) 0 null))
  (set `self.k2A_screenTxtrParam` _returnvalue))